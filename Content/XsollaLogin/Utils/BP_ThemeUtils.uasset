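; Blueprint utility functions that apply Xsolla Login UI themes to widgets.
; Color and font getters look up named entries in the theme, returning a caller-supplied default when the theme is invalid.
; Style updaters rebuild input field and button styles from named state brushes, keeping existing padding and other untouched settings.
; Input fields also take themed font and text color with an explicit size; both updaters do nothing without a valid theme.
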(fn GetThemeColor
  (params (Theme :type Xsolla%20Utils%20Theme%20Class%20Reference) (ColorName :type String) (DefaultColor :type Slate%20Color%20Structure))
  (bind _returnvalue (Class|XsollaUtilsLibrary|GetTheme Theme))
  (if (Utilities|IsValid _returnvalue)
    (return (Utilities|Struct|MakeSlateColor (Math|Conversions|ToLinearColor(Color) (Class|XsollaUtilsTheme|GetColor _returnvalue ColorName))))
    (else
      (return DefaultColor))))

(fn GetThemeFont
  (params (Theme :type Xsolla%20Utils%20Theme%20Class%20Reference) (FontName :type String) (DefaultFont :type Slate%20Font%20Info%20Structure))
  (bind _returnvalue (Class|XsollaUtilsLibrary|GetTheme Theme))
  (if (Utilities|IsValid _returnvalue)
    (return (Class|XsollaUtilsTheme|GetFont _returnvalue FontName))
    (else
      (return DefaultFont))))

(fn UpdateInputFieldStyle
  (params (Theme :type Xsolla%20Utils%20Theme%20Class%20Reference) (NormalStateBrush :type String) (HoverStateBrush :type String) (ActiveStateBrush :type String) (DisabledStateBrush :type String) (FontName :type String) (FontSize :type Integer) (TextColor :type String) (InputField :type Editable%20Text%20Box%20Object%20Reference))
  (bind _returnvalue (Class|XsollaUtilsLibrary|GetTheme Theme))
  (bind _slatefontinfo (Utilities|Struct|MakeSlateFontInfo "/Game/XsollaLogin/Common/Assets/Font/Font_Roboto-Regular.Font_Roboto-Regular" 0 "(OutlineSize=0,bSeparateFillAlpha=False,bApplyOutlineToDropShadows=False,OutlineMaterial=None,OutlineColor=(R=0.000000,G=0.000000,B=0.000000,A=1.000000))" "None" 14))
  (bind _returnvalue_2 (Themes|GetThemeFont Theme FontName _slatefontinfo))
  (bind (_fontobject _fontmaterial _outlinesettings _typefacefontname _size _letterspacing) (Utilities|Struct|BreakSlateFontInfo _returnvalue_2))
  (Utilities|IsValid _returnvalue
    (:Is%20Valid
      (Variables|/Script/UMG.EditableTextBox|SetWidgetStyle InputField (Utilities|Struct|MakeEditableTextBoxStyle (Class|XsollaUtilsTheme|GetBrush _returnvalue NormalStateBrush) (Class|XsollaUtilsTheme|GetBrush _returnvalue HoverStateBrush) (Class|XsollaUtilsTheme|GetBrush _returnvalue ActiveStateBrush) (Class|XsollaUtilsTheme|GetBrush _returnvalue DisabledStateBrush) (.Padding (Utilities|Struct|BreakEditableTextBoxStyle (Variables|/Script/UMG.EditableTextBox|GetWidgetStyle InputField))) (Utilities|Struct|MakeSlateFontInfo _fontobject _fontmaterial _outlinesettings _typefacefontname FontSize _letterspacing) (Themes|GetThemeColor Theme TextColor (Utilities|Struct|MakeSlateColor "(R=1.000000,G=1.000000,B=1.000000,A=0.700000)")) (.BackgroundColor (Utilities|Struct|BreakEditableTextBoxStyle (Variables|/Script/UMG.EditableTextBox|GetWidgetStyle InputField))) (.ReadOnlyForegroundColor (Utilities|Struct|BreakEditableTextBoxStyle (Variables|/Script/UMG.EditableTextBox|GetWidgetStyle InputField))) (.HScrollBarPadding (Utilities|Struct|BreakEditableTextBoxStyle (Variables|/Script/UMG.EditableTextBox|GetWidgetStyle InputField))) (.VScrollBarPadding (Utilities|Struct|BreakEditableTextBoxStyle (Variables|/Script/UMG.EditableTextBox|GetWidgetStyle InputField))) (.ScrollBarStyle (Utilities|Struct|BreakEditableTextBoxStyle (Variables|/Script/UMG.EditableTextBox|GetWidgetStyle InputField))))))))

(fn UpdateButtonStyle
  (params (Theme :type Xsolla%20Utils%20Theme%20Class%20Reference) (NormalStateBrush :type String) (HoverStateBrush :type String) (PressedStateBrush :type String) (DisabledStateBrush :type String) (Button :type Button%20Object%20Reference))
  (bind _returnvalue (Class|XsollaUtilsLibrary|GetTheme Theme))
  (bind _widgetstyle (Variables|/Script/UMG.Button|GetWidgetStyle Button))
  (bind (_normal _hovered _pressed _disabled _normalpadding _pressedpadding _pressedslatesound _hoveredslatesound) (Utilities|Struct|BreakButtonStyle _widgetstyle))
  (Utilities|IsValid _returnvalue
    (:Is%20Valid
      (Class|Button|SetStyle Button (Utilities|Struct|MakeButtonStyle (Class|XsollaUtilsTheme|GetBrush _returnvalue NormalStateBrush) (Class|XsollaUtilsTheme|GetBrush _returnvalue HoverStateBrush) (Class|XsollaUtilsTheme|GetBrush _returnvalue PressedStateBrush) (Class|XsollaUtilsTheme|GetBrush _returnvalue DisabledStateBrush) _normalpadding _pressedpadding _pressedslatesound _hoveredslatesound)))))